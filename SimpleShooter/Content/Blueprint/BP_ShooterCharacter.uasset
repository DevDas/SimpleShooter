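; Player shooter character Blueprint with switchable camera views, movement speed modifiers and a crosshair widget created on BeginPlay.
; V toggles the Camera and FPP components and records IsFPSView, while holding LeftAlt stops the SpringArm inheriting yaw.
; ADS halves walk speed while held and sets EquipWeapon on press and release, which gates a temporary LeftShift double-speed sprint.
; Tick prints Health and MaxHealth as debug output.
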(event `self.ReceiveBeginPlay`
  (bind _returnvalue (`|CreateWidget` "/Game/UI/WBP_Crosshair.WBP_Crosshair_C"))
  (`UserWidget.AddToViewport` _returnvalue 0))

(event `Key|LeftAlt`
  (params (Key :type "Key Structure"))
  (bind _springarm (`self.SpringArm`))
  (:`Pressed`
    (set `SpringArmComponent.bInheritYaw` false _springarm))
  (:`Released`
    (set `SpringArmComponent.bInheritYaw` true _springarm)))

(event `Key|V`
  (params (Key :type "Key Structure"))
  (bind _fpp (`self.FPP`))
  (:`Pressed`
    (`ActorComponent.ToggleActive` (`self.Camera`))
    (`ActorComponent.ToggleActive` _fpp)
    (set `self.IsFPSView` (`ActorComponent.IsActive` _fpp))))

(event `self.ReceiveTick`
  (params (DeltaSeconds :type "Float (single-precision)"))
  (`KismetSystemLibrary.PrintString` (`KismetStringLibrary.Conv_DoubleToString` (`self.Health`)) true true (struct :`G` 0.66 :`B` 1.0 :`A` 1.0) 0.0)
  (`KismetSystemLibrary.PrintString` (`KismetStringLibrary.Conv_DoubleToString` (`self.MaxHealth`)) true true (struct :`R` 1.0 :`G` 0.097454 :`A` 1.0) 0.0))

(event `Key|LeftShift`
  (params (Key :type "Key Structure"))
  (bind _charactermovement (`self.CharacterMovement`))
  (bind _maxwalkspeed (`CharacterMovementComponent.MaxWalkSpeed` _charactermovement))
  ;[1 1 1] Temporary Setup : We Will Fix In Future
  (:`Pressed`
    (if (`self.EquipWeapon`)
      (set `CharacterMovementComponent.MaxWalkSpeed` (* _maxwalkspeed 2.0) _charactermovement)))
  (:`Released`
    (if (`self.EquipWeapon`)
      (set `CharacterMovementComponent.MaxWalkSpeed` (/ _maxwalkspeed 2.0) _charactermovement))))

(event `Key|B`
  (params (Key :type "Key Structure"))
  ;[1 1 1] Temporary Setup : We Will Fix In Future
)

(event `Key|N`
  (params (Key :type "Key Structure"))
  ;[1 1 1] Temporary Setup : We Will Fix In Future
)

(event `InputAction|ADS`
  (params (Key :type "Key Structure"))
  (bind _charactermovement (`self.CharacterMovement`))
  (bind _maxwalkspeed (`CharacterMovementComponent.MaxWalkSpeed` _charactermovement))
  ;[1 1 1] Temporary Setup : We Will Fix In Future
  (:`Pressed`
    (set `self.EquipWeapon` true)
    (set `CharacterMovementComponent.MaxWalkSpeed` (/ _maxwalkspeed 2.0) _charactermovement))
  (:`Released`
    (set `self.EquipWeapon` true)
    (set `CharacterMovementComponent.MaxWalkSpeed` (* _maxwalkspeed 2.0) _charactermovement)))

(fn `UserConstructionScript`)