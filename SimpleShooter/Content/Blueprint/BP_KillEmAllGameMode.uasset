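; BP_KillEmAllGameMode is a game mode Blueprint with logic for switching to a spectator view when the player dies.
; BeginPlay fetches the player's shooter character and controller through a cast helper, but the OnDead binding is disconnected, so nothing here hooks up the death handler.
; That handler calls BlendView, which cubically blends the controller's view target to a random SpecView actor in the level.
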(event `self.ReceiveBeginPlay`
  (bind (_pawn _pawncontroller) (`self.CastPlayerAndController`)))

(event `OnDead_Event_0`
  (`self.BlendView` (stale `self.ReceiveBeginPlay` _pawncontroller)))

(fn `BlendView`
  (params (PlayerController :type "PlayerController Object Reference"))
  (bind _outactors (`GameplayStatics.GetAllActorsOfClass` "/Game/Blueprint/SpecView.SpecView_C"))
  (`PlayerController.SetViewTargetWithBlend` PlayerController (`|GetArrayItem` _outactors (`KismetMathLibrary.RandomIntegerInRange` 0 (- (`KismetArrayLibrary.Array_Length` _outactors) 1))) 2.0 "VTBlend_Cubic" 0.0 false))

(fn `CastPlayerAndController`
  (returns (Pawn :type "/Game/Blueprint/BP_ShooterCharacter Object Reference") (PawnController :type "PlayerController Object Reference"))
  (bind _asbp_shooter_character (cast `/Game/Blueprint/BP_ShooterCharacter` (`GameplayStatics.GetPlayerPawn` 0)))
  (bind _asbp_player_controller (cast `/Game/Blueprint/BP_PlayerController` (`Pawn.GetController` _asbp_shooter_character)))
  (return _asbp_shooter_character _asbp_player_controller))

(fn `UserConstructionScript`)